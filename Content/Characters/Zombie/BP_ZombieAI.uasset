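; Zombie character that chases and attacks the player once it is inside the lab, driven by BP_ZombieAIController and BT_Zombie.
; BeginPlay links player and controller and writes InRoom to the blackboard; Tick also calls RunBehaviorTree every frame.
; While alive, paired DoOnce nodes toggle Attack and Chase modes by horizontal player distance.
; Capsule hits from "attack"-tagged components trigger Death mode, and UpdateSpeed sets walk and fly speeds.
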(event `self.ReceiveBeginPlay`
  (`|ExecutionSequence`
    (:`then_0`
      ;[1 1 1] 초기화
      (bind _asbp_player_character (cast `/Game/Characters/BP_PlayerCharacter` (`GameplayStatics.GetPlayerCharacter` 0)))
      (bind _output_get (set `self.Player Character` _asbp_player_character))
      (bind _asbp_zombie_aicontroller (cast `/Game/Characters/Zombie/BP_ZombieAIController` (`AIBlueprintHelperLibrary.GetAIController` self)))
      (bind _output_get_2 (set `self.Zombie Controller` _asbp_zombie_aicontroller))
      (set `/Game/Characters/Zombie/BP_ZombieAIController.Player Character` _output_get _output_get_2))
    (:`then_1`
      ;[1 1 1] Zombie가 연구실 내로 들어왔는지 (수정 예정)
      (`BlackboardComponent.SetValueAsBool` (`AIBlueprintHelperLibrary.GetBlackboard` null) (`self.InRoom`) (`self.Is In Room?`)))))

(event `self.ReceiveTick`
  (params (DeltaSeconds :type "Float (single-precision)"))
  (bind _zombie_controller (`self.Zombie Controller`))
  (`|ExecutionSequence`
    (:`then_0`
      (if (and (`self.Is In Room?`) (!= (`BlackboardComponent.GetValueAsEnum` (`AIBlueprintHelperLibrary.GetBlackboard` null) (`self.ZombieState`)) 4))
        (if (< (`self.GetHorizontalDistanceTo` (`self.Player Character`)) 100.0)
          (`/Engine/EditorBlueprintResources/StandardMacros.DoOnce` false :!label _label
            (:`Completed`
              (`/Game/Characters/Zombie/BP_ZombieAIController.Set Attack Mode` _zombie_controller)
              (goto _label_2 :!via `Reset`)))
          (else
            (`/Engine/EditorBlueprintResources/StandardMacros.DoOnce` false :!label _label_2
              (:`Completed`
                (`/Game/Characters/Zombie/BP_ZombieAIController.Set Chase Mode` _zombie_controller)
                (goto _label :!via `Reset`)))))))
    (:`then_1`
      (`AIController.RunBehaviorTree` (`self.Zombie Controller`) "/Game/Characters/Zombie/BT_Zombie.BT_Zombie"))))

(event `self.CapsuleComponent.OnComponentHit`
  (params (HitComponent :type "PrimitiveComponent Object Reference") (OtherActor :type "Actor Object Reference") (OtherComp :type "PrimitiveComponent Object Reference") (NormalImpulse :type "Vector Structure") (Hit :type "HitResult Structure (by ref)"))
  (if (`ActorComponent.ComponentHasTag` OtherComp "attack")
    (`KismetSystemLibrary.PrintString` "2")
    (`/Game/Characters/Zombie/BP_ZombieAIController.Set Death Mode` (`self.Zombie Controller`))))

(fn `Update Speed`
  (params (Speed :type "Float (double-precision)"))
  (bind _charactermovement (`self.CharacterMovement`))
  (set `CharacterMovementComponent.MaxWalkSpeed` Speed _charactermovement)
  (set `CharacterMovementComponent.MaxFlySpeed` Speed _charactermovement))

(fn `UserConstructionScript`)
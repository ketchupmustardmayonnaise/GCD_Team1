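; BP_ZombieCharacter is an enemy zombie that pursues the player character, which it caches on BeginPlay.
; Each Tick, while not in the Death state, it switches between Chase and Attack based on 2D distance to the player and an attack range.
; Chase feeds the horizontal direction toward the player straight into AddMovementInput, without pathfinding.
; Only Chase has behavior here; Attack just stops that movement input.
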(event `self.ReceiveBeginPlay`
  ;[1 1 1] Target이 될 Player Character 초기화
  (bind _asbp_player_character (cast `/Game/Characters/BP_PlayerCharacter` (`GameplayStatics.GetPlayerCharacter` 0)))
  (set `self.CharacterInstance` _asbp_player_character))

(event `self.ReceiveTick`
  (params (DeltaSeconds :type "Float (single-precision)"))
  (bind (_returnvalue_x _returnvalue_y) (`KismetMathLibrary.BreakVector2D` (- (`KismetMathLibrary.Conv_VectorToVector2D` (`self.K2_GetActorLocation` (`self.CharacterInstance`))) (`KismetMathLibrary.Conv_VectorToVector2D` (`self.K2_GetActorLocation`)))))
  (`|ExecutionSequence`
    (:`then_0`
      ;[1 1 1] 좀비가 살아있다면
      (if (`|EnumInequality` (`self.ZombieState`) "NewEnumerator3")
        ;[1 1 1] 캐릭터까지의 거리 계산
        (set `self.DistanceToCharacter` (`KismetMathLibrary.Distance2D` (`KismetMathLibrary.Conv_VectorToVector2D` (`self.K2_GetActorLocation`)) (`KismetMathLibrary.Conv_VectorToVector2D` (`self.K2_GetActorLocation` (`self.CharacterInstance`)))))
        ;[1 1 1] 캐릭터까지의 거리를 기반으로 state 결정
        (if (< (`self.DistanceToCharacter`) (`self.AttackDistance`))
          (set `self.ZombieState` "NewEnumerator2")
          (else
            (set `self.ZombieState` "NewEnumerator1")))))
    (:`then_1`
      (switch `/Game/Characters/Zombie/ZombieState` (`self.ZombieState`)
        (:`NewEnumerator1`
          ;[1 1 1] Chase Player Character
          (`self.AddMovementInput` (`KismetMathLibrary.Conv_Vector2DToVector` (`KismetMathLibrary.MakeVector2D` _returnvalue_x _returnvalue_y))))))))

(event `self.ReceiveActorBeginOverlap`
  (params (OtherActor :type "Actor Object Reference")))

(fn `UserConstructionScript`)
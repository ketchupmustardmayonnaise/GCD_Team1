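; AI controller for zombie characters that runs their behavior tree and switches them between idle, chase, attack and climb modes.
; On possess it caches the zombie and its AnimBP, stores the level's climb actor in the Blackboard, runs BT_Zombie and enters chase.
; Mode events write the Blackboard state and matching animation state together.
; Perception-based player detection is disconnected, leaving its update handler empty.
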(event `self.ReceivePossess`
  (params (PossessedPawn :type "Pawn Object Reference"))
  ;[1 1 1] 초기화
  (`|ExecutionSequence`
    (:`then_0`
      (bind _asbp_zombie_ai (cast `/Game/Characters/Zombie/BP_ZombieAI` PossessedPawn))
      (bind _output_get (set `self.Zombie Character` _asbp_zombie_ai))
      (bind _asabp_zombie (cast `/Game/Characters/Zombie/ABP_Zombie` (`SkeletalMeshComponent.GetAnimInstance` (`Character.Mesh` _output_get))))
      (set `self.Zombie Anim` _asabp_zombie)
      (bind _returnvalue (`GameplayStatics.GetActorOfClass` "/Game/Animations/Procedural/BP_ClimbActor.BP_ClimbActor_C"))
      (`BlackboardComponent.SetValueAsObject` (`AIBlueprintHelperLibrary.GetBlackboard` null) (`self.ActorToClimb`) _returnvalue))
    (:`then_1`
      (`self.RunBehaviorTree` "/Game/Characters/Zombie/BT_Zombie.BT_Zombie")
      (`self.Set Chase Mode`))))

(event `Set Idle Mode`
  ;[1 1 1] Set Behavior Tree
  (`BlackboardComponent.SetValueAsObject` (`self.Blackboard`) (`self.PlayerActor`) null)
  (`BlackboardComponent.SetValueAsEnum` (`self.Blackboard`) (`self.ZombieState`) 0) ; 0: Idle
  (set `/Game/Characters/Zombie/ABP_Zombie.Anim State` "NewEnumerator0" (`self.Zombie Anim`)))

(event `Set Climb Mode`
  ;[1 1 1] Set Behavior Tree
  (`BlackboardComponent.SetValueAsEnum` (`self.Blackboard`) (`self.ZombieState`) 5) ; 5: Climb
  (set `/Game/Characters/Zombie/ABP_Zombie.Anim State` "NewEnumerator5" (`self.Zombie Anim`)))

(event `Set Chase Mode`
  ;[1 1 1] Set Behavior Tree
  (`BlackboardComponent.SetValueAsObject` (`self.Blackboard`) (`self.PlayerActor`) (`self.Player Character`))
  (`BlackboardComponent.SetValueAsEnum` (`self.Blackboard`) (`self.ZombieState`) 1) ; 1: Chase
  (set `/Game/Characters/Zombie/ABP_Zombie.Anim State` "NewEnumerator1" (`self.Zombie Anim`)))

(event `Set Attack Mode`
  ;[1 1 1] Set Behavior Tree
  (`BlackboardComponent.SetValueAsObject` (`self.Blackboard`) (`self.PlayerActor`) (`self.Player Character`))
  (`BlackboardComponent.SetValueAsEnum` (`self.Blackboard`) (`self.ZombieState`) 2) ; 2: Attack
  (set `/Game/Characters/Zombie/ABP_Zombie.Anim State` "NewEnumerator2" (`self.Zombie Anim`)))

(event `self.AIPerception.OnTargetPerceptionUpdated`
  (params (Actor :type "Actor Object Reference") (Stimulus :type "AIStimulus Structure"))
  ;[1 1 1] Timer (일단 의미 없는 듯 나중에 사용하게 되면 수정하기...)
)

(event `StartPlayerTimer`
  ;[1 1 1] Timer (일단 의미 없는 듯 나중에 사용하게 되면 수정하기...)
  (set `self.Player Character` null))

(fn `UserConstructionScript`)